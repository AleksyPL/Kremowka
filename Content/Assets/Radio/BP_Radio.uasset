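; BP_Radio is an interactable radio that alternates between playing random songs and stopping on each Interactions event via a FlipFlop.
; TurnOn loops up to Max, setting and playing a random Songs entry, with a Delay inside the loop leading to PlayNext for another random pick.
; The Delay's duration comes from a separate random index, not necessarily the playing song.
; TurnOff only stops Audio, leaving any pending Delay active.
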(event `self.Interactions`
  (params (Player :type "Character Object Reference"))
  (`/Engine/EditorBlueprintResources/StandardMacros.FlipFlop`
    (:`A`
      (`self.Turn On`))
    (:`B`
      (`self.Turn Off`))))

(event `Turn On`
  (bind _audio (`self.Audio`))
  (bind _max (`self.Max`))
  (bind _output (`|GetArrayItem` (`self.Songs`) (`KismetMathLibrary.RandomInteger` _max)))
  (for _ (range (+ _max 1))
    (`AudioComponent.SetSound` _audio _output)
    (`AudioComponent.Play` _audio 0.0)
    (`KismetSystemLibrary.Delay` (`SoundBase.Duration` _output))
    (`self.PlayNext`)))

(event `Turn Off`
  (`AudioComponent.Stop` (`self.Audio`)))

(event `PlayNext`
  (bind _audio (`self.Audio`))
  (`AudioComponent.SetSound` _audio (`|GetArrayItem` (`self.Songs`) (`KismetMathLibrary.RandomInteger` (`self.Max`))))
  (`AudioComponent.Play` _audio 0.0))

(fn `UserConstructionScript`)