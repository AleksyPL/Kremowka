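; BP_GenericItem is the parent actor for pickable items that go into the player's inventory.
; On BeginPlay it fills a missing ItemObject from GetDefaulItemObejct, which returns nothing here, presumably for child classes to override.
; Interaction offers the ItemObject to the player's InventoryComponent.
; On success it deselects and destroys itself, clears the InteractionComponent's selected actor and removes interaction widgets.
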(event `self.ReceiveBeginPlay`
  (if (not (`KismetSystemLibrary.IsValid` (`self.ItemObject`)))
    (bind _itemobject (`self.GetDefaulItemObejct`))
    (set `self.ItemObject` _itemobject)))

(event `/Game/Blueprints/MainCharacter/Interactions/BP_Select_Interaction.Interactions`
  (params (Player :type "Character Object Reference"))
  (`self.AddItemToIventory` Player))

(fn `AddItemToIventory`
  (params (Object :type "Object Object Reference"))
  (bind _asmain_character_movement (cast `/Game/Blueprints/MainCharacter/MainCharacterMovement` Object))
  (bind _added (`/Game/UI/Inventory/InventoryComponent.TryAddItem` (`/Game/Blueprints/MainCharacter/MainCharacterMovement.InventoryComponent` _asmain_character_movement) (`self.ItemObject`)))
  (if _added
    (message `/Game/Blueprints/MainCharacter/Interactions/BP_Select_Interaction.DeselectMyActor` self)
    (`self.K2_DestroyActor`)
    (bind _asmain_character_movement_2 (cast `/Game/Blueprints/MainCharacter/MainCharacterMovement` (`GameplayStatics.GetPlayerCharacter` 0)))
    (set `/Game/Blueprints/MainCharacter/Interactions/InteractionComponent.SelectedActor` null (`/Game/Blueprints/MainCharacter/MainCharacterMovement.InteractionComponent` _asmain_character_movement_2))
    (bind _foundwidgets (`WidgetBlueprintLibrary.GetAllWidgetsOfClass` "/Game/Blueprints/MainCharacter/Interactions/Widget_Interaction.Widget_Interaction_C"))
    (`Widget.RemoveFromParent` _foundwidgets)))

(fn `GetDefaulItemObejct`
  (returns (ItemObject :type "/Game/Items/PickableItemParentClass/BP_GenericItemObject Object Reference"))
  (return null))

(fn `IsSelected`
  (returns (IsSelected :type Boolean))
  (return false))

(fn `UserConstructionScript`)