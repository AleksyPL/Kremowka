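; BP_GenericItemObject is a data object for a pickable item, exposing its dimensions, icon and item class through getter functions.
; GetImage returns either the normal or the rotated UI icon depending on the rotation flag.
; Dimensions and ItemClass are returned directly, which suggests use by a grid-style inventory UI.
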(fn `GetDimensions`
  (returns (Dimensions :type "IntPoint Structure"))
  (return (`self.Dimensions`)))

(fn `GetImage`
  (returns (ReturnValue :type "MaterialInterface Object Reference"))
  (return (select `bool` (`self.Rotaded`) :`false` (`self.UIIcon`) :`true` (`self.UIIconRotated`))))

(fn `GetItemClass`
  (returns (ItemClass :type "/Game/Items/PickableItemParentClass/BP_GenericItem Class Reference"))
  (return (`self.ItemClass`)))