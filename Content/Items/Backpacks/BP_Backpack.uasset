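; BP_Backpack is a backpack item that the player equips by interacting with it.
; The Interactions event calls Equip, which runs EquipBackpack to store this actor as the Backpack reference on the InventoryComponent of player 0's MainCharacterMovement character.
; It does not attach or hide the actor, and IsSelected always returns false.
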(event `Equip`
  (`self.EquipBackpack`))

(event `/Game/Blueprints/MainCharacter/Inventory/BP_Select_Interaction.Interactions`
  (params (Player :type "Character Object Reference"))
  (`self.Equip`))

(fn `EquipBackpack`
  (set `/Game/UI/Inventory/InventoryComponent.Backpack` self (`/Game/Blueprints/MainCharacter/MainCharacterMovement.InventoryComponent` (cast `/Game/Blueprints/MainCharacter/MainCharacterMovement` (`GameplayStatics.GetPlayerCharacter` 0) :!pure true))))

(fn `IsSelected`
  (returns (IsSelected :type Boolean))
  (return false))

(fn `UserConstructionScript`)