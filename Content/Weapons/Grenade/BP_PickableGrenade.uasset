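; BP_PickableGrenade is a pickable M67 grenade item that describes how it is represented as an inventory-style item.
; GetDefaulItemObejct constructs a BP_GenericItemObject with a single-cell size, normal and rotated M67 icons, and this Blueprint as its item class.
; The event graph holds only disabled stubs, and the construction script just calls the parent, so the class adds no other behavior in its graphs.
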(fn `GetDefaulItemObejct`
  (returns (ItemObject :type "/Game/Items/PickableItemParentClass/BP_GenericItemObject Object Reference"))
  (bind _returnvalue (`|GenericCreateObject` self "/Game/Items/PickableItemParentClass/BP_GenericItemObject.BP_GenericItemObject_C" (make `IntPoint` 1 1) "/Game/Materials/M_M67GrenadeIcon.M_M67GrenadeIcon" "/Game/Materials/M_M67GrenadeIcon_Rotated.M_M67GrenadeIcon_Rotated" "BP_PickableGrenade_C"))
  (return _returnvalue))

(fn `UserConstructionScript`
  (`parent.UserConstructionScript`))