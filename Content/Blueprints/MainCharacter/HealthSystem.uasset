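; HealthSystem holds hit points for the main character and enemies and handles damage between them.
; CurrentHP starts at MaxHP on BeginPlay, and RecieveDamage subtracts damage, clamps at zero and prints the damaged actor's name with its remaining HP.
; GiveDamage casts the target to MainCharacterMovement or Enemy and forwards the damage to that actor's own HealthSystem, ignoring other actor types.
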(event `self.ReceiveBeginPlay`
  (set `self.CurrentHP` (`self.MaxHP`)))

(fn `GiveDamage`
  (params (DamageToGive :type "Float (double-precision)") (ActorToDamage :type "Actor Object Reference"))
  (bind _asmain_character_movement (cast `/Game/Blueprints/MainCharacter/MainCharacterMovement` ActorToDamage)
    (:`then`
      (`self.RecieveDamage` (`/Game/Blueprints/MainCharacter/MainCharacterMovement.HealthSystem` _asmain_character_movement) DamageToGive _asmain_character_movement))
    (:`CastFailed`
      (bind _asenemy (cast `/Game/Blueprints/Enemies/Enemy` ActorToDamage))
      (`self.RecieveDamage` (`/Game/Blueprints/Enemies/Enemy.HealthSystem` _asenemy) DamageToGive _asenemy))))

(fn `RecieveDamage`
  (params (RecievedDamage :type "Float (double-precision)") (DamagedActor :type "Actor Object Reference"))
  (bind _returnvalue (- (`self.CurrentHP`) RecievedDamage))
  (if (< _returnvalue 0.0)
    (bind _output_get (set `self.CurrentHP` 0.0))
    (else
      (set `self.CurrentHP` _returnvalue)))
  (`KismetSystemLibrary.PrintString` (`KismetStringLibrary.Concat_StrStr` (`KismetSystemLibrary.GetObjectName` (`local.DamagedActor`)) " - " (`KismetStringLibrary.Conv_DoubleToString` _output_get))))